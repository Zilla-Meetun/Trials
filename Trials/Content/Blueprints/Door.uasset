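; Door Blueprint that swings open on Activate and closes on Deactivate.
; An Open timeline drives the door component's relative yaw, playing forward to open and reversing to close.
; When the timeline finishes, a check on the DIsplayed flag and the first Dialogue entry gates setting that flag and passing Dialogue to the BP_Zilly player character for display.
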(event EventBeginPlay)

(event Collision|EventActorBeginOverlap
  (params (OtherActor :type Actor%20Object%20Reference)))

(event EventTick
  (params (DeltaSeconds :type Float%20%28single-precision%29)))

(event EventActivate
  (bind _dialogue (Variables|Default|GetDialogue))
  (bind _rotationvalue (Timeline|Open Play)
    (:Update
      (Transformation|SetRelativeRotation (Variables|Default|GetDoor) (Math|Rotator|MakeRotator 0.0 0.0 _rotationvalue) false false))
    (:Finished
      (if (not (Math|Boolean|ANDBoolean (not (Variables|Default|GetbDIsplayed)) (Utilities|Array|IsValidIndex _dialogue) (Utilities|Text|TextIsEmpty (Utilities|Array|Get(acopy) _dialogue))))
        (Variables|Default|SetbDIsplayed true)
        (bind _asbp_zilly (Utilities|Casting|CastToBP_Zilly (Game|GetPlayerCharacter 0)))
        (Default|ShowDialogue _asbp_zilly (Variables|Default|GetDialogue))))))

(event EventDeactivate
  (bind _dialogue (Variables|Default|GetDialogue))
  (bind _rotationvalue (Timeline|Open Reverse)
    (:Update
      (Transformation|SetRelativeRotation (Variables|Default|GetDoor) (Math|Rotator|MakeRotator 0.0 0.0 _rotationvalue) false false))
    (:Finished
      (if (not (Math|Boolean|ANDBoolean (not (Variables|Default|GetbDIsplayed)) (Utilities|Array|IsValidIndex _dialogue) (Utilities|Text|TextIsEmpty (Utilities|Array|Get(acopy) _dialogue))))
        (Variables|Default|SetbDIsplayed true)
        (bind _asbp_zilly (Utilities|Casting|CastToBP_Zilly (Game|GetPlayerCharacter 0)))
        (Default|ShowDialogue _asbp_zilly (Variables|Default|GetDialogue))))))

(fn ConstructionScript)