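; BP_Tile is a tile actor that shows its on or off state through a colour parameter on a dynamic material created at BeginPlay.
; FlipTile inverts IsOn and updates the colour.
; Collider overlap enters a DoOnce that ResetFlip re-arms, but nothing follows it.
; Disconnected logic would flip the tile and its Neighbours in Lights Out fashion, with a delay and reset inside the loop.
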(event OnComponentBeginOverlap(TileCollider)
  (params (OverlappedComponent :type Primitive%20Component%20Object%20Reference) (OtherActor :type Actor%20Object%20Reference) (OtherComp :type Primitive%20Component%20Object%20Reference) (OtherBodyIndex :type Integer) (bFromSweep :type Boolean) (SweepResult :type Hit%20Result%20Structure%20%28by%20ref%29))
  (Utilities|FlowControl|DoOnce false))

(event Custom|ResetFlip
  (Utilities|FlowControl|DoOnce false) ; enters at Reset
)

(event EventBeginPlay
  (bind _returnvalue (Rendering|Material|CreateDynamicMaterialInstance (Variables|Default|GetTile) 0 0 "None" :!class /Script/Engine.PrimitiveComponent))
  (Variables|Default|SetTileMat _returnvalue)
  (if (Variables|Default|GetbIsOn)
    (Rendering|Material|SetVectorParameterValue (Variables|Default|GetTileMat) "Colour" (Variables|Default|GetOnColour) :!class /Script/Engine.MaterialInstanceDynamic)
    (else
      (Rendering|Material|SetVectorParameterValue (Variables|Default|GetTileMat) "Colour" (Variables|Default|GetOffColour) :!class /Script/Engine.MaterialInstanceDynamic))))

(fn ConstructionScript)

(fn FlipTile
  (bind _tilemat (Variables|Default|GetTileMat))
  (bind _output_get (Variables|Default|SetbIsOn (not (Variables|Default|GetbIsOn))))
  (if _output_get
    (Rendering|Material|SetVectorParameterValue _tilemat "Colour" (Variables|Default|GetOnColour) :!class /Script/Engine.MaterialInstanceDynamic)
    (else
      (Rendering|Material|SetVectorParameterValue _tilemat "Colour" (Variables|Default|GetOffColour) :!class /Script/Engine.MaterialInstanceDynamic))))