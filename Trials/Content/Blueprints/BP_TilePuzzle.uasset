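; Tile puzzle actor that sends an activation message once every tile in its grid is on.
; The construction script spawns BP_Tile child actors in a spaced grid and links orthogonal neighbours by flat-array index.
; Neighbour math strides by XLength although tiles are stored in YLength-long runs, so links are correct only for square grids.
; IsComplete checks all tiles, fires Activation, then marks each tile as finished.
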(fn ConstructionScript
  (bind _grid (Variables|Default|GetGrid))
  (bind _grid_2 (Variables|Default|GetGrid))
  (bind _grid_3 (Variables|Default|GetGrid))
  (bind _grid_4 (Variables|Default|GetGrid))
  (Utilities|Array|Clear (Variables|Default|GetGrid))
  (for _index (range 1 (Variables|Default|GetXLength))
    (for _index_2 (range 1 (Variables|Default|GetYLength))
      (bind _returnvalue (AddComponent|AddChildActorComponent false (Math|Transform|MakeTransform (Math|Vector|MakeVector (* _index (Variables|Default|GetSpacing)) (* _index_2 (Variables|Default|GetSpacing)) 0.0) "0, 0, 0" "1,1,1")))
      (bind _asbp_tile (Utilities|Casting|CastToBP_Tile (Variables|/Script/Engine.ChildActorComponent|GetChildActor _returnvalue)))
      (Utilities|Array|Clear (Variables|/Game/Blueprints/BP_Tile.BP_Tile_C|GetNeighbours _asbp_tile))
      (Utilities|Array|Add (Variables|Default|GetGrid) _asbp_tile)))
  (for (_array_element _array_index) (Variables|Default|GetGrid)
    (if (and (Utilities|Array|IsValidIndex _grid_4 (- _array_index 1)) (!= (Math|Integer|%(Integer) _array_index (Variables|Default|GetXLength)) 0))
      (Utilities|Array|Add (Variables|/Game/Blueprints/BP_Tile.BP_Tile_C|GetNeighbours _array_element) (Utilities|Array|Get(acopy) _grid_4 (- _array_index 1))))
    (if (and (Utilities|Array|IsValidIndex _grid (+ _array_index 1)) (!= (Math|Integer|%(Integer) _array_index (Variables|Default|GetXLength)) (- (Variables|Default|GetXLength) 1)))
      (Utilities|Array|Add (Variables|/Game/Blueprints/BP_Tile.BP_Tile_C|GetNeighbours _array_element) (Utilities|Array|Get(acopy) _grid (+ _array_index 1))))
    (if (Utilities|Array|IsValidIndex _grid_2 (- _array_index (Variables|Default|GetXLength)))
      (Utilities|Array|Add (Variables|/Game/Blueprints/BP_Tile.BP_Tile_C|GetNeighbours _array_element) (Utilities|Array|Get(acopy) _grid_2 (- _array_index (Variables|Default|GetXLength)))))
    (if (Utilities|Array|IsValidIndex _grid_3 (+ _array_index (Variables|Default|GetXLength)))
      (Utilities|Array|Add (Variables|/Game/Blueprints/BP_Tile.BP_Tile_C|GetNeighbours _array_element) (Utilities|Array|Get(acopy) _grid_3 (+ _array_index (Variables|Default|GetXLength)))))))

(fn IsComplete
  (Variables|Default|SetComplete true)
  (bind _array_element (Utilities|Array|ForEachLoopwithBreak (Variables|Default|GetGrid) :!label _label)
    (:LoopBody
      (if (not (Variables|/Game/Blueprints/BP_Tile.BP_Tile_C|GetbIsOn _array_element))
        (Variables|Default|SetComplete (Variables|/Game/Blueprints/BP_Tile.BP_Tile_C|GetbIsOn _array_element))
        (goto _label Break)))
    (:Completed
      (if (Variables|Default|GetComplete)
        (Class|ITrigger|Activate(Message) (Variables|Default|GetActivation))
        (for _array_element_2 (Variables|Default|GetGrid)
          (Variables|/Game/Blueprints/BP_Tile.BP_Tile_C|SetbPuzzleFinished _array_element_2 true))))))