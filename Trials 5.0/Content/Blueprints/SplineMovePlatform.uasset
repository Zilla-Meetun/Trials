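; A platform actor that moves a static mesh along its Path spline, started and stopped by Activate and Deactivate.
; The SplineMovement timeline's value scales the spline length to set the mesh's local location.
; On finishing, it waits one second and replays from the start, unless MovesOnce has stopped it near the 0.5 track value.
; The MoveRate play-rate setting is unconnected and never runs.
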(event Custom|Finished
  (bind _path (Variables|Default|GetPath))
  (Utilities|FlowControl|Delay 1.0)
  (bind _newtrack_0 (Timeline|SplineMovement PlayFromStart)
    (:Update
      (if (Variables|Default|GetbIsActive)
        (if (and (Math|Float|NearlyEqual(Float) _newtrack_0 0.5 0.005) (Variables|Default|GetbMovesOnce))
          (Timeline|SplineMovement Stop)
          (else
            (Transformation|SetRelativeLocation (Variables|Default|GetStaticMesh) (Spline|GetLocationatDistanceAlongSpline _path (* _newtrack_0 (Spline|GetSplineLength _path)) "Local") false false)))
        (else
          (Timeline|SplineMovement Stop))))
    (:Finished
      (CallFunction|Finished))))

(event EventBeginPlay)

(event Collision|EventActorBeginOverlap
  (params (OtherActor :type Actor%20Object%20Reference)))

(event EventTick
  (params (DeltaSeconds :type Float%20%28single-precision%29)))

(event EventActivate
  (bind _path (Variables|Default|GetPath))
  (Variables|Default|SetbIsActive true)
  (bind _newtrack_0 (Timeline|SplineMovement Play)
    (:Update
      (if (Variables|Default|GetbIsActive)
        (if (and (Math|Float|NearlyEqual(Float) _newtrack_0 0.5 0.005) (Variables|Default|GetbMovesOnce))
          (Timeline|SplineMovement Stop)
          (else
            (Transformation|SetRelativeLocation (Variables|Default|GetStaticMesh) (Spline|GetLocationatDistanceAlongSpline _path (* _newtrack_0 (Spline|GetSplineLength _path)) "Local") false false)))
        (else
          (Timeline|SplineMovement Stop))))
    (:Finished
      (CallFunction|Finished))))

(event EventDeactivate
  (bind _path (Variables|Default|GetPath))
  (Variables|Default|SetbIsActive false)
  (bind _newtrack_0 (Timeline|SplineMovement Stop)
    (:Update
      (if (Variables|Default|GetbIsActive)
        (if (and (Math|Float|NearlyEqual(Float) _newtrack_0 0.5 0.005) (Variables|Default|GetbMovesOnce))
          (Timeline|SplineMovement Stop)
          (else
            (Transformation|SetRelativeLocation (Variables|Default|GetStaticMesh) (Spline|GetLocationatDistanceAlongSpline _path (* _newtrack_0 (Spline|GetSplineLength _path)) "Local") false false)))
        (else
          (Timeline|SplineMovement Stop))))
    (:Finished
      (CallFunction|Finished))))

(fn ConstructionScript)