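; Moving platform actor that animates its static mesh along a timeline-driven path.
; The PlatformLocation timeline's vector track, scaled by per-axis offsets, sets the mesh's relative location while IsActive is true.
; Activate and Deactivate set that flag and play or stop the timeline, with Activate also printing a debug string.
; On completion, the Finished event restarts the timeline from the start after a short delay, looping the motion.
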(event Custom|Finished
  (Utilities|FlowControl|Delay 1.0)
  (bind _newtrack_0 (Timeline|PlatformLocation PlayFromStart)
    (:Update
      (if (Variables|Default|GetbIsActive)
        (Transformation|SetRelativeLocation (Variables|Default|GetStaticMesh) (Math|Vector|MakeVector (* (.x _newtrack_0) (Variables|Default|GetXOffset)) (* (.y _newtrack_0) (Variables|Default|GetYOffset)) (* (.z _newtrack_0) (Variables|Default|GetZOffset))) false false)
        (else
          (Timeline|PlatformLocation Stop))))
    (:Finished
      (CallFunction|Finished))))

(event EventBeginPlay)

(event Collision|EventActorBeginOverlap
  (params (OtherActor :type Actor%20Object%20Reference)))

(event EventTick
  (params (DeltaSeconds :type Float%20%28single-precision%29)))

(event EventActivate
  (Development|PrintString "Hello")
  (Variables|Default|SetbIsActive true)
  (bind _newtrack_0 (Timeline|PlatformLocation Play)
    (:Update
      (if (Variables|Default|GetbIsActive)
        (Transformation|SetRelativeLocation (Variables|Default|GetStaticMesh) (Math|Vector|MakeVector (* (.x _newtrack_0) (Variables|Default|GetXOffset)) (* (.y _newtrack_0) (Variables|Default|GetYOffset)) (* (.z _newtrack_0) (Variables|Default|GetZOffset))) false false)
        (else
          (Timeline|PlatformLocation Stop))))
    (:Finished
      (CallFunction|Finished))))

(event EventDeactivate
  (Variables|Default|SetbIsActive false)
  (bind _newtrack_0 (Timeline|PlatformLocation Stop)
    (:Update
      (if (Variables|Default|GetbIsActive)
        (Transformation|SetRelativeLocation (Variables|Default|GetStaticMesh) (Math|Vector|MakeVector (* (.x _newtrack_0) (Variables|Default|GetXOffset)) (* (.y _newtrack_0) (Variables|Default|GetYOffset)) (* (.z _newtrack_0) (Variables|Default|GetZOffset))) false false)
        (else
          (Timeline|PlatformLocation Stop))))
    (:Finished
      (CallFunction|Finished))))

(fn ConstructionScript)