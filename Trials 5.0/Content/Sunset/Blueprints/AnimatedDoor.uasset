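; AnimatedDoor is a double door that swings open or shut each time its Activate event fires.
; Activate flips the DoorClosed flag, playing the DoorRotation timeline forward when it becomes true and reversing it otherwise.
; The timeline's DoorOpen track drives the yaw of DoorL and DoorR in opposite directions, holding each leaf at a fixed relative offset either side of center.
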(event EventActivate
  (bind _output_get (Variables|Default|SetDoorClosed (not (Variables|Default|GetDoorClosed))))
  (if _output_get
    (bind _door_open (Timeline|Door%20Rotation Play)
      (:Update
        (Transformation|SetRelativeLocationAndRotation (Variables|Default|GetDoorL) "-80.000000, 0, 0" (Math|Rotator|MakeRotator 0.0 0.0 _door_open) false false)
        (Transformation|SetRelativeLocationAndRotation (Variables|Default|GetDoorR) "80.000000, 0, 0" (* (Math|Rotator|MakeRotator 0.0 0.0 _door_open) -1.0) false false)))
    (else
      (Timeline|Door%20Rotation Reverse))))

(fn ConstructionScript)